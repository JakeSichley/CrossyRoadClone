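; Railroad crossing actor that repeatedly spawns trains and runs warning lights and sound, starting once the player's X position comes within range.
; Tick starts a randomized SpawnCar timer, then flags an incoming train shortly before it fires, playing the warning once and alternating two point lights through a delayed FlipFlop.
; When the spawned BP_Train passes a Y threshold, the lights switch off and a new random spawn timer starts.
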(event Custom|SpawnCar
  ;[1 1 1] Spawn Train
  (bind _returnvalue (Game|SpawnActorfromClass "/Game/Blueprints/cars/BP_Train.BP_Train_C" (Math|Transform|MakeTransform (.location (Transformation|GetWorldTransform (Variables|Default|GetCarSpawnPoint))) "0, 0, 0" "1,1,1") "Undefined" self 0))
  (Default|SetDirection _returnvalue true)
  (Variables|Default|SetTrain _returnvalue))

(event Custom|TrainComing
  ;[1 1 1] Railroad lights
  (Utilities|FlowControl|Sequence
    (:then_0
      (Utilities|FlowControl|DoOnce false
        (:Completed
          (Audio|SpawnSoundAttached "/Game/Sounds/RailroadWarning.RailroadWarning" (Variables|Default|GetPointLightRight) "None" "0, 0, 0" "0, 0, 0" "KeepRelativeOffset" false 0.5 1.0 0.0 0 0))))
    (:then_1
      (Utilities|FlowControl|Delay 0.25)
      (Utilities|FlowControl|FlipFlop
        (:A
          (Rendering|SetVisibility (Variables|Default|GetPointLightLeft) true false)
          (Rendering|SetVisibility (Variables|Default|GetPointLightRight) false false))
        (:B
          (Rendering|SetVisibility (Variables|Default|GetPointLightLeft) false false)
          (Rendering|SetVisibility (Variables|Default|GetPointLightRight) true false))))))

(event EventBeginPlay
  ;[1 1 1] Begin
  (|CallParentFunction)
  (Rendering|SetVisibility (Variables|Default|GetPointLightRight) false false)
  (Rendering|SetVisibility (Variables|Default|GetPointLightLeft) false false)
  (Variables|Default|SetIsTrainComing false))

(event EventTick
  (params (DeltaSeconds :type Float%20%28single-precision%29))
  (bind _train (Variables|Default|GetTrain))
  (bind _defaultsceneroot (Variables|Default|GetDefaultSceneRoot))
  ;[1 1 1] Main update
  (|CallParentFunction DeltaSeconds)
  (Utilities|FlowControl|Sequence
    (:then_0
      (Utilities|IsValid _defaultsceneroot
        (:Is%20Valid
          (if (< (- (.x (Transformation|GetWorldLocation _defaultsceneroot)) (.x (Transformation|GetWorldLocation (Variables|/Game/Blueprints/BP_Player.BP_Player_C|GetBox (Variables|Default|GetPlayer))))) 2.2e+02)
            (Utilities|FlowControl|DoOnce false
              (:Completed
                (bind _returnvalue (Utilities|Time|SetTimerbyFunctionName self "SpawnCar" (Math|Random|RandomFloatinRange 4.0 9.0)))
                (Variables|Default|SetSpawnCarTimer _returnvalue)))))))
    (:then_1
      (if (and (Utilities|Time|IsTimerActivebyHandle (Variables|Default|GetSpawnCarTimer)) (< (Utilities|Time|GetTimerRemainingTimebyHandle (Variables|Default|GetSpawnCarTimer)) 1.5))
        (Utilities|FlowControl|DoOnce false :!label _label
          (:Completed
            (Variables|Default|SetIsTrainComing true)
            ;[1 1 1] Railroad lights
            (Utilities|FlowControl|DoOnce false) ; enters at Reset
          ))))
    (:then_2
      (if (and (and (Utilities|Time|IsTimerActivebyHandle (Variables|Default|GetSpawnCarTimer)) (< (Utilities|Time|GetTimerRemainingTimebyHandle (Variables|Default|GetSpawnCarTimer)) 1.5)) (Variables|Default|GetIsTrainComing))
        (CallFunction|TrainComing)))
    (:then_3
      (Utilities|IsValid _train
        (:Is%20Valid
          (if (<= (.y (Transformation|GetActorLocation _train)) -8e+02)
            (Variables|Default|SetIsTrainComing false)
            (Rendering|SetVisibility (Variables|Default|GetPointLightLeft) false false)
            (Rendering|SetVisibility (Variables|Default|GetPointLightRight) false false)
            (Utilities|Time|ClearandInvalidateTimerbyHandle (Variables|Default|GetSpawnCarTimer))
            (bind _returnvalue_2 (Utilities|Time|SetTimerbyFunctionName self "SpawnCar" (Math|Random|RandomFloatinRange 7.0 13.0)))
            (Variables|Default|SetSpawnCarTimer _returnvalue_2)
            (goto _label Reset)))))))

(fn ConstructionScript
  (|CallParentFunction))