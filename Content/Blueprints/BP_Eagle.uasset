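; BP_Eagle is an eagle that chases the player and appears to snatch their chicken.
; From BeginPlay, Tick moves the eagle mesh toward player pawn 0 at constant interpolation speed, without sweeping.
; Overlapping BP_Player ends the chase and hides the player's ChickenMesh, after which Tick moves the eagle steadily upward by re-targeting a point above its current location each frame.
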(event OnComponentBeginOverlap(EagleMesh)
  (params (OverlappedComponent :type Primitive%20Component%20Object%20Reference) (OtherActor :type Actor%20Object%20Reference) (OtherComp :type Primitive%20Component%20Object%20Reference) (OtherBodyIndex :type Integer) (bFromSweep :type Boolean) (SweepResult :type Hit%20Result%20Structure%20%28by%20ref%29))
  (bind _asbp_player (Utilities|Casting|CastToBP_Player OtherActor))
  (Variables|Default|SetIsChasing false)
  (Rendering|SetVisibility (Variables|/Game/Blueprints/BP_Player.BP_Player_C|GetChickenMesh _asbp_player) false false))

(event EventTick
  (params (DeltaSeconds :type Float%20%28single-precision%29))
  (bind _eaglemesh (Variables|Default|GetEagleMesh))
  (bind _eaglemesh_2 (Variables|Default|GetEagleMesh))
  (bind _returnvalue (Transformation|GetWorldLocation _eaglemesh_2))
  (if (Variables|Default|GetIsChasing)
    (Transformation|SetWorldLocation _eaglemesh (Math|Interpolation|VInterptoConstant (Transformation|GetWorldLocation _eaglemesh) (Transformation|GetActorLocation (Game|Player|GetPlayerPawn 0)) DeltaSeconds 2.5e+02) false false)
    (else
      (Transformation|SetWorldLocation (Variables|Default|GetEagleMesh) (Math|Interpolation|VInterptoConstant _returnvalue (+ _returnvalue "0, 0,400.000000") DeltaSeconds 2.5e+02) false false))))

(event EventBeginPlay
  (Variables|Default|SetIsChasing true))

(fn ConstructionScript)