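; Lane spawner actor that lays down a starting chain of BP_GrassLane actors on BeginPlay.
; The first lane spawns just below the player pawn, and each following one at the NextSpawnPoint of the previous lane, tracked as NewestLane.
; SpawnLaneAtSpawnPoint extends the chain by one lane.
; The assignment of this spawner to the lane's GrassSpawner is disconnected, so lanes receive no back-reference here.
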(event EventBeginPlay
  (CallFunction|SpawnInitialLanes))

(event Collision|EventActorBeginOverlap
  (params (OtherActor :type Actor%20Object%20Reference)))

(event EventTick
  (params (DeltaSeconds :type Float%20%28single-precision%29)))

(fn ConstructionScript)

(fn SpawnLane
  (params (SpawnLocation :type Vector))
  (bind _returnvalue (Game|SpawnActorfromClass "/Game/Blueprints/BP_GrassLane.BP_GrassLane_C" (Math|Transform|MakeTransform SpawnLocation "0, 0, 0" "1,1,1") "Undefined" 0 0))
  (bind _output_get (Variables|Default|SetNewestLane _returnvalue)))

(fn SpawnLaneatSpawnPoint
  (CallFunction|SpawnLane (Transformation|GetWorldLocation (Variables|/Game/Blueprints/BP_GrassLane.BP_GrassLane_C|GetNextSpawnPoint (Variables|Default|GetNewestLane)))))

(fn SpawnInitialLanes
  (bind _returnvalue (Game|Player|GetPlayerPawn 0))
  (bind _returnvalue_2 (Transformation|GetActorLocation _returnvalue))
  (for _index (range 0 3)
    (Utilities|IsValid (Variables|Default|GetNewestLane)
      (:Is%20Valid
        (CallFunction|SpawnLaneatSpawnPoint))
      (:Is%20Not%20Valid
        (CallFunction|SpawnLane (Math|Vector|MakeVector (.x _returnvalue_2) (.y _returnvalue_2) (+ (.z _returnvalue_2) -2e+01)))))))