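; BP_Car1 is a traffic car that squashes the player's chicken on contact.
; BeginPlay randomizes speed, flips the mesh if MoveRight is set and attaches an engine sound.
; Tick drives it along local -Y, randomly triggers a one-time honk and destroys it outside world Y bounds.
; Side and front collision overlaps with a living BP_Player call X or Z squash respectively, then play an impact sound.
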(event OnComponentBeginOverlap(SideCollision)
  (params (OverlappedComponent :type Primitive%20Component%20Object%20Reference) (OtherActor :type Actor%20Object%20Reference) (OtherComp :type Primitive%20Component%20Object%20Reference) (OtherBodyIndex :type Integer) (bFromSweep :type Boolean) (SweepResult :type Hit%20Result%20Structure%20%28by%20ref%29))
  (bind _asbp_player (Utilities|Casting|CastToBP_Player OtherActor))
  (bind _isalive (Default|IsAlive _asbp_player))
  (if _isalive
    (Default|GetSquashedX _asbp_player)
    (CallFunction|SpawnSound)))

(event OnComponentBeginOverlap(SideCollision1)
  (params (OverlappedComponent :type Primitive%20Component%20Object%20Reference) (OtherActor :type Actor%20Object%20Reference) (OtherComp :type Primitive%20Component%20Object%20Reference) (OtherBodyIndex :type Integer) (bFromSweep :type Boolean) (SweepResult :type Hit%20Result%20Structure%20%28by%20ref%29))
  (bind _asbp_player (Utilities|Casting|CastToBP_Player OtherActor))
  (bind _isalive (Default|IsAlive _asbp_player))
  (if _isalive
    (Default|GetSquashedX _asbp_player)
    (CallFunction|SpawnSound)))

(event OnComponentBeginOverlap(FrontCollision)
  (params (OverlappedComponent :type Primitive%20Component%20Object%20Reference) (OtherActor :type Actor%20Object%20Reference) (OtherComp :type Primitive%20Component%20Object%20Reference) (OtherBodyIndex :type Integer) (bFromSweep :type Boolean) (SweepResult :type Hit%20Result%20Structure%20%28by%20ref%29))
  (bind _asbp_player (Utilities|Casting|CastToBP_Player OtherActor))
  (bind _isalive (Default|IsAlive _asbp_player))
  (if _isalive
    (Default|GetSquashedZ _asbp_player)
    (CallFunction|SpawnSound)))

(event EventBeginPlay
  ;[1 1 1] Set The static mesh for car models
  (CallFunction|RandomizeSpeed)
  (Audio|SpawnSoundAttached "/Game/Sounds/EngineTest.EngineTest" (Variables|Default|GetCarMesh) "None" "0, 0, 0" "0, 0, 0" "KeepRelativeOffset" false 0.75 1.0 0.0 "/Game/Sounds/CarDynamic.CarDynamic" 0))

(event Collision|EventActorBeginOverlap
  (params (OtherActor :type Actor%20Object%20Reference)))

(event EventTick
  (params (DeltaSeconds :type Float%20%28single-precision%29))
  (bind _returnvalue (Transformation|GetActorLocation))
  (Utilities|FlowControl|Sequence
    (:then_0
      (Transformation|AddActorLocalOffset (Math|Vector|MakeVector 0.0 (* (Variables|Default|GetSpeed) DeltaSeconds -1.0) 0.0) false false))
    (:then_1
      (if (== 200 (Math|Random|RandomInteger 500))
        (Utilities|FlowControl|DoOnce false
          (:Completed
            (Audio|SpawnSoundAttached "/Game/Sounds/CarHonk.CarHonk" (Variables|Default|GetCarMesh) "None" "0, 0, 0" "0, 0, 0" "KeepRelativeOffset" true 1.0 1.0 0.0 "/Game/Sounds/HonkAttenuation.HonkAttenuation" 0)))))
    (:then_2
      (if (or (< (.y _returnvalue) -1e+03) (> (.y _returnvalue) 1e+03))
        (Actor|DestroyActor)))))

(fn ConstructionScript)

(fn RandomizeSpeed
  (Variables|Default|SetSpeed (Math|Conversions|ToFloat(Integer) (Math|Random|RandomIntegerinRange 80 100)))
  (if (Variables|Default|GetMoveRight)
    (Transformation|SetRelativeRotation (Variables|Default|GetCarMesh) "0,180.000000, 0" false false)))

(fn SetDirection
  (params (DirectionRight :type Boolean))
  (Variables|Default|SetMoveRight DirectionRight))

(fn SpawnSound
  (Audio|SpawnSoundAttached "/Game/Sounds/ChickenImpact.ChickenImpact" (Variables|Default|GetCarMesh) "None" "0, 0, 0" "0, 0, 0" "KeepRelativeOffset" true 0.5 1.0 0.0 0 0))