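; BP_Train is a moving train hazard that calls Explode on any BP_Player overlapping its collision.
; It plays an attached passing sound at spawn, moves along its local Y axis by Speed each tick, and destroys itself once its head leaves a fixed world-Y range.
; SetDirection negates Speed in either case and also rotates the head when Left is false.
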(event OnComponentBeginOverlap(Collision)
  (params (OverlappedComponent :type Primitive%20Component%20Object%20Reference) (OtherActor :type Actor%20Object%20Reference) (OtherComp :type Primitive%20Component%20Object%20Reference) (OtherBodyIndex :type Integer) (bFromSweep :type Boolean) (SweepResult :type Hit%20Result%20Structure%20%28by%20ref%29))
  (bind _asbp_player (Utilities|Casting|CastToBP_Player OtherActor))
  (Default|Explode _asbp_player))

(event EventBeginPlay
  (Audio|SpawnSoundAttached "/Game/Sounds/TrainPassing.TrainPassing" (Variables|Default|GetTrainHead) "None" "0, 0, 0" "0, 0, 0" "KeepRelativeOffset" false 0.5 1.0 0.0 0 0))

(event EventTick
  (params (DeltaSeconds :type Float%20%28single-precision%29))
  (bind _trainhead (Variables|Default|GetTrainHead))
  (bind _returnvalue (Transformation|GetWorldLocation _trainhead))
  (Utilities|FlowControl|Sequence
    (:then_0
      (Transformation|AddActorLocalOffset (Math|Vector|MakeVector 0.0 (* (Variables|Default|GetSpeed) DeltaSeconds) 0.0) false false))
    (:then_1
      (if (or (< (.y _returnvalue) -1e+03) (> (.y _returnvalue) 1e+03))
        (Actor|DestroyActor)))))

(fn ConstructionScript)

(fn SetDirection
  (params (Left :type Boolean))
  (if Left
    _
    (else
      (Transformation|SetRelativeRotation (Variables|Default|GetTrainHead) "0,180.000000, 0" false false)))
  (Variables|Default|SetSpeed (* (Variables|Default|GetSpeed) -1.0)))