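; BP_Car is a traffic car obstacle that drives across the world and squashes BP_Player on contact.
; BeginPlay picks one of four vehicle meshes and a random speed, turning only the mesh when MoveRight, set through SetDirection, is true.
; Tick moves it along local negative Y and destroys it beyond the world Y bounds.
; Side collisions squash the player on X, the front collision on Z.
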(event OnComponentBeginOverlap(SideCollision)
  (params (OverlappedComponent :type Primitive%20Component%20Object%20Reference) (OtherActor :type Actor%20Object%20Reference) (OtherComp :type Primitive%20Component%20Object%20Reference) (OtherBodyIndex :type Integer) (bFromSweep :type Boolean) (SweepResult :type Hit%20Result%20Structure%20%28by%20ref%29))
  (bind _asbp_player (Utilities|Casting|CastToBP_Player OtherActor))
  (Default|GetSquashedX _asbp_player))

(event OnComponentBeginOverlap(SideCollision1)
  (params (OverlappedComponent :type Primitive%20Component%20Object%20Reference) (OtherActor :type Actor%20Object%20Reference) (OtherComp :type Primitive%20Component%20Object%20Reference) (OtherBodyIndex :type Integer) (bFromSweep :type Boolean) (SweepResult :type Hit%20Result%20Structure%20%28by%20ref%29))
  (bind _asbp_player (Utilities|Casting|CastToBP_Player OtherActor))
  (Default|GetSquashedX _asbp_player))

(event OnComponentBeginOverlap(FrontCollision)
  (params (OverlappedComponent :type Primitive%20Component%20Object%20Reference) (OtherActor :type Actor%20Object%20Reference) (OtherComp :type Primitive%20Component%20Object%20Reference) (OtherBodyIndex :type Integer) (bFromSweep :type Boolean) (SweepResult :type Hit%20Result%20Structure%20%28by%20ref%29))
  (bind _asbp_player (Utilities|Casting|CastToBP_Player OtherActor))
  (Default|GetSquashedZ _asbp_player))

(event EventBeginPlay
  (Components|StaticMesh|SetStaticMesh (Variables|Default|GetCarMesh) (Utilities|Select :Index (Math|Random|RandomIntegerinRange 0 3) :Option%200 "/Game/Models/Cars/car.car" :Option%201 "/Game/Models/Cars/truck.truck" :Option%202 "/Game/Models/Cars/van.van" :Option%203 "/Game/Models/Cars/car2.car2"))
  (CallFunction|RandomizeSpeed))

(event Collision|EventActorBeginOverlap
  (params (OtherActor :type Actor%20Object%20Reference)))

(event EventTick
  (params (DeltaSeconds :type Float%20%28single-precision%29))
  (bind _returnvalue (Transformation|GetActorLocation))
  (Utilities|FlowControl|Sequence
    (:then_0
      (Transformation|AddActorLocalOffset (Math|Vector|MakeVector 0.0 (* (Variables|Default|GetSpeed) DeltaSeconds -1.0) 0.0) false false))
    (:then_1
      (if (or (< (.y _returnvalue) -1e+03) (> (.y _returnvalue) 1e+03))
        (Actor|DestroyActor)))))

(fn ConstructionScript)

(fn RandomizeSpeed
  (if (Variables|Default|GetMoveRight)
    (Variables|Default|SetSpeed (Math|Conversions|ToFloat(Integer) (Math|Random|RandomIntegerinRange 80 100)))
    (Transformation|SetRelativeRotation (Variables|Default|GetCarMesh) "0.000000,180.000000,0.000000" false false)
    (else
      (Variables|Default|SetSpeed (Math|Conversions|ToFloat(Integer) (Math|Random|RandomIntegerinRange 80 100))))))

(fn SetDirection
  (params (DirectionRight :type Boolean))
  (Variables|Default|SetMoveRight DirectionRight))