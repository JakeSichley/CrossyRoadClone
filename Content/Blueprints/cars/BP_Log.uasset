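; BP_Log is a moving log actor that carries the player along when they touch it.
; Each tick it moves along its local Y axis, opposite to the sign of Speed, and destroys itself once its world Y position leaves a fixed range.
; When LogMesh hits a BP_Player, it shifts that player's Box by the same frame step in world Y, with sweep enabled.
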(event OnComponentHit(LogMesh)
  (params (HitComponent :type Primitive%20Component%20Object%20Reference) (OtherActor :type Actor%20Object%20Reference) (OtherComp :type Primitive%20Component%20Object%20Reference) (NormalImpulse :type Vector :default "0, 0, 0") (Hit :type Hit%20Result%20Structure%20%28by%20ref%29))
  (bind _asbp_player (Utilities|Casting|CastToBP_Player OtherActor))
  (Transformation|AddWorldOffset (Variables|/Game/Blueprints/BP_Player.BP_Player_C|GetBox _asbp_player) (Math|Vector|MakeVector 0.0 (* (Variables|Default|GetSpeed) (Utilities|Time|GetWorldDeltaSeconds) -1.0) 0.0) true false))

(event EventTick
  (params (DeltaSeconds :type Float%20%28single-precision%29))
  (bind _returnvalue (Transformation|GetActorLocation))
  (Utilities|FlowControl|Sequence
    (:then_0
      (Transformation|AddActorLocalOffset (Math|Vector|MakeVector 0.0 (* (Variables|Default|GetSpeed) DeltaSeconds -1.0) 0.0) false false))
    (:then_1
      (if (or (< (.y _returnvalue) -1e+03) (> (.y _returnvalue) 1e+03))
        (Actor|DestroyActor)))))

(fn ConstructionScript)