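; BP_Lane is a self-recycling lane segment that extends the track as the player advances along X.
; When BP_Player overlaps its TriggerZone, it calls LaneSpawner to spawn a lane at the spawn point, then destroys the trigger so it fires once.
; It finds the player on BeginPlay and checks each Tick, destroying itself once the player's Box is a fixed X distance past the lane's root.
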(event OnComponentBeginOverlap(TriggerZone)
  (params (OverlappedComponent :type Primitive%20Component%20Object%20Reference) (OtherActor :type Actor%20Object%20Reference) (OtherComp :type Primitive%20Component%20Object%20Reference) (OtherBodyIndex :type Integer) (bFromSweep :type Boolean) (SweepResult :type Hit%20Result%20Structure%20%28by%20ref%29))
  (Utilities|Casting|CastToBP_Player OtherActor)
  (Default|SpawnLaneatSpawnPoint (Variables|Default|GetLaneSpawner))
  (Components|DestroyComponent (Variables|Default|GetTriggerZone)))

(event EventBeginPlay
  (bind _returnvalue (Actor|GetActorOfClass "/Game/Blueprints/BP_Player.BP_Player_C"))
  (Variables|Default|SetPlayer _returnvalue))

(event EventTick
  (params (DeltaSeconds :type Float%20%28single-precision%29))
  (if (> (- (.x (Transformation|GetWorldLocation (Variables|/Game/Blueprints/BP_Player.BP_Player_C|GetBox (Variables|Default|GetPlayer)))) (.x (Transformation|GetWorldLocation (Variables|Default|GetDefaultSceneRoot)))) 2.6e+02)
    (Actor|DestroyActor)))

(fn ConstructionScript)