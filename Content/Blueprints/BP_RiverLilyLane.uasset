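; River lane with randomly scattered lily pads, where bound volumes flush the player away to either side.
; On BeginPlay it attempts up to four lily pad meshes on a 40-unit grid, some with an attached BP_Coin.
; The duplicate check, stored slot and pad position each roll separately, so pads can overlap.
; River overlap only prints "Splash"; the player's Drown call is disconnected.
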(event OnComponentBeginOverlap(River)
  (params (OverlappedComponent :type Primitive%20Component%20Object%20Reference) (OtherActor :type Actor%20Object%20Reference) (OtherComp :type Primitive%20Component%20Object%20Reference) (OtherBodyIndex :type Integer) (bFromSweep :type Boolean) (SweepResult :type Hit%20Result%20Structure%20%28by%20ref%29))
  (bind _asbp_player (Utilities|Casting|CastToBP_Player OtherActor))
  (Development|PrintString "Splash"))

(event OnComponentBeginOverlap(RightBound)
  (params (OverlappedComponent :type Primitive%20Component%20Object%20Reference) (OtherActor :type Actor%20Object%20Reference) (OtherComp :type Primitive%20Component%20Object%20Reference) (OtherBodyIndex :type Integer) (bFromSweep :type Boolean) (SweepResult :type Hit%20Result%20Structure%20%28by%20ref%29))
  (bind _asbp_player (Utilities|Casting|CastToBP_Player OtherActor))
  (Default|FlushAway _asbp_player true))

(event OnComponentBeginOverlap(LeftBound)
  (params (OverlappedComponent :type Primitive%20Component%20Object%20Reference) (OtherActor :type Actor%20Object%20Reference) (OtherComp :type Primitive%20Component%20Object%20Reference) (OtherBodyIndex :type Integer) (bFromSweep :type Boolean) (SweepResult :type Hit%20Result%20Structure%20%28by%20ref%29))
  (bind _asbp_player (Utilities|Casting|CastToBP_Player OtherActor))
  (Default|FlushAway _asbp_player false))

(event EventBeginPlay
  (|CallParentFunction)
  (CallFunction|SpawnLilypads))

(fn ConstructionScript)

(fn SpawnLilypads
  (bind _returnvalue (Math|Random|RandomIntegerinRange -4 4))
  (for _index (range 0 (Math|Random|RandomIntegerinRange 0 3))
    (if (not (Utilities|Array|ContainsItem (LocalVariables|GetSpawnLocations) _returnvalue))
      (Utilities|Array|SetArrayElem (LocalVariables|GetSpawnLocations) _index _returnvalue true)
      (bind _returnvalue_2 (AddComponent|AddStaticMeshComponent false (Math|Transform|MakeTransform (Math|Vector|MakeVector 2e+01 (* _returnvalue 4e+01) 0.0) "0, 0, 0" "1,1,1")))
      (if (Math|Float|InRange(Float) (Math|Random|RandomFloatinRange 0.0 1e+01) 3.0 5.0)
        (bind _returnvalue_3 (Game|SpawnActorfromClass "/Game/Blueprints/items/BP_Coin.BP_Coin_C" (Math|Transform|MakeTransform "0.000000,0.0,4.000000" "0, 0, 0" "1,1,1") "Undefined" 0 0))
        (Transformation|AttachComponentToComponent _returnvalue_3 _returnvalue_2 "None" "KeepRelative" "KeepRelative" "KeepRelative" false)))))