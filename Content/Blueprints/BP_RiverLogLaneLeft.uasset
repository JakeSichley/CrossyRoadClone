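; River lane actor for a Crossy Road-style crossing game, spawning moving logs and handling player deaths in the water.
; On BeginPlay it picks one random log speed, starts water ambience and begins a self-repeating spawn loop with random delays.
; Overlapping the river drowns the player with a splash sound, while side bounds flush the player away.
; Logs leaving the left bound, or found under a player entering it, switch to a fixed fast speed.
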(event OnComponentEndOverlap(LeftBound)
  (params (OverlappedComponent :type Primitive%20Component%20Object%20Reference) (OtherActor :type Actor%20Object%20Reference) (OtherComp :type Primitive%20Component%20Object%20Reference) (OtherBodyIndex :type Integer))
  (bind _asbp_log (Utilities|Casting|CastToBP_Log OtherActor))
  (Variables|/Game/Blueprints/cars/BP_Log.BP_Log_C|SetSpeed _asbp_log -4e+02))

(event OnComponentBeginOverlap(River)
  (params (OverlappedComponent :type Primitive%20Component%20Object%20Reference) (OtherActor :type Actor%20Object%20Reference) (OtherComp :type Primitive%20Component%20Object%20Reference) (OtherBodyIndex :type Integer) (bFromSweep :type Boolean) (SweepResult :type Hit%20Result%20Structure%20%28by%20ref%29))
  ;[1 1 1] Kill player
  (bind _asbp_player (Utilities|Casting|CastToBP_Player OtherActor))
  (Development|PrintString "Splash")
  (Default|Drown _asbp_player)
  (Audio|SpawnSoundAttached "/Game/Sounds/ChickenWaterImpact.ChickenWaterImpact" (Variables|Default|GetRiver) "None" "0, 0, 0" "0, 0, 0" "KeepRelativeOffset" true 1.0 1.0 0.0 0 0))

(event OnComponentBeginOverlap(RightBound)
  (params (OverlappedComponent :type Primitive%20Component%20Object%20Reference) (OtherActor :type Actor%20Object%20Reference) (OtherComp :type Primitive%20Component%20Object%20Reference) (OtherBodyIndex :type Integer) (bFromSweep :type Boolean) (SweepResult :type Hit%20Result%20Structure%20%28by%20ref%29))
  ;[1 1 1] Kill player
  (bind _asbp_player (Utilities|Casting|CastToBP_Player OtherActor))
  (Default|FlushAway _asbp_player true))

(event OnComponentBeginOverlap(LeftBound)
  (params (OverlappedComponent :type Primitive%20Component%20Object%20Reference) (OtherActor :type Actor%20Object%20Reference) (OtherComp :type Primitive%20Component%20Object%20Reference) (OtherBodyIndex :type Integer) (bFromSweep :type Boolean) (SweepResult :type Hit%20Result%20Structure%20%28by%20ref%29))
  ;[1 1 1] Kill player
  (bind _asbp_player (Utilities|Casting|CastToBP_Player OtherActor))
  (Default|FlushAway _asbp_player false)
  (bind _asbp_log (Utilities|Casting|CastToBP_Log (Utilities|Array|Get(acopy) (Collision|GetOverlappingActors _asbp_player "/Game/Blueprints/cars/BP_Log.BP_Log_C" :!class /Script/Engine.Actor))))
  (Variables|/Game/Blueprints/cars/BP_Log.BP_Log_C|SetSpeed _asbp_log -4e+02))

(event Custom|SpawnLog
  ;[1 1 1] Spawn Log
  (bind _returnvalue (Game|SpawnActorfromClass "/Game/Blueprints/cars/BP_Log.BP_Log_C" (Transformation|GetWorldTransform (Variables|Default|GetLogSpawnPoint)) "AlwaysSpawn" self 0))
  (Default|SetDirection _returnvalue true)
  (Default|SetSpeed _returnvalue (Variables|Default|GetLogSpeed))
  (Utilities|FlowControl|Delay (Math|Random|RandomFloatinRange 1.8 4.0))
  (CallFunction|SpawnLog))

(event EventBeginPlay
  (|CallParentFunction)
  (Variables|Default|SetLogSpeed (Math|Random|RandomFloatinRange 4e+01 8e+01))
  (CallFunction|SpawnLog)
  (Audio|SpawnSoundAttached "/Game/Sounds/WaterAmbient.WaterAmbient" (Variables|Default|GetRiver) "None" "0, 0, 0" "0, 0, 0" "KeepRelativeOffset" true 0.25 1.0 0.0 "/Game/Sounds/Ambient.Ambient" 0))

(fn ConstructionScript)