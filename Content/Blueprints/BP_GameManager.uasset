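; Game manager that tracks steps, coins and high score, drives the HUD, pause and restart widgets, and handles level restart.
; BeginPlay builds the widgets, loads high score and coins from the save slot, and starts a countdown that calls SpawnEagle on the player.
; Each step resets that countdown, so idling too long triggers the eagle.
; Showing the restart screen writes high score and coins back, creating the save if missing.
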(event EventBeginPlay
  (bind _returnvalue (Game|GetPlayerController 0))
  (Utilities|FlowControl|Sequence
    (:then_0
      (bind _returnvalue_2 (UserInterface|CreateWidget "/Game/UI/WBP_HUD.WBP_HUD_C"))
      (UserInterface|Viewport|AddtoViewport _returnvalue_2 0)
      (Variables|/Game/UI/WBP_HUD.WBP_HUD_C|SetGameManager _returnvalue_2 self)
      (bind _output_get (Variables|Default|SetHUDWidget _returnvalue_2))
      (bind _returnvalue_3 (SaveGame|LoadGamefromSlot "save_data"))
      (bind _asbp_save_game (Utilities|Casting|CastToBP_SaveGame _returnvalue_3)
        (:then
          (Variables|Default|SetHiScore (Variables|/Game/Blueprints/BP_SaveGame.BP_SaveGame_C|GetHiScore _asbp_save_game))
          (Variables|Default|SetCoins (Variables|/Game/Blueprints/BP_SaveGame.BP_SaveGame_C|GetCoins _asbp_save_game)))
        (:CastFailed
          _))
      (Default|UpdateStepText _output_get)
      (Default|UpdateCoinText _output_get)
      (Default|UpdateHiScore _output_get))
    (:then_1
      (bind _returnvalue_4 (UserInterface|CreateWidget "/Game/UI/WBP_Restart.WBP_Restart_C"))
      (Variables|Default|SetRestartWidget _returnvalue_4))
    (:then_2
      (bind _returnvalue_5 (UserInterface|CreateWidget "/Game/UI/WBP_Pause.WBP_Pause_C"))
      (Variables|Default|SetPauseWidget _returnvalue_5))
    (:then_3
      (bind _returnvalue_6 (Actor|GetActorOfClass "/Game/Blueprints/BP_Player.BP_Player_C"))
      (Variables|Default|SetPlayer _returnvalue_6)
      (Input|SetInputModeGameOnly _returnvalue)
      (Variables|/Script/Engine.PlayerController|SetbShowMouseCursor _returnvalue false))
    (:then_4
      (bind _returnvalue_7 (Utilities|Time|SetTimerbyFunctionName (Variables|Default|GetPlayer) "SpawnEagle" (Variables|Default|GetTimeLimit)))
      (Variables|Default|SetCountdownTimer _returnvalue_7))))

(fn ConstructionScript)

(fn IncreaseStep
  (bind _steps (Variables|Default|GetSteps))
  (Math|Integer|IncrementInt (Variables|Default|GetSteps)
    (:%20%20
      (Utilities|FlowControl|Sequence
        (:then_0
          (Default|UpdateStepText (Variables|Default|GetHUDWidget))
          (Utilities|Time|ClearandInvalidateTimerbyHandle (Variables|Default|GetCountdownTimer))
          (bind _returnvalue (Utilities|Time|SetTimerbyFunctionName (Variables|Default|GetPlayer) "SpawnEagle" (Variables|Default|GetTimeLimit)))
          (Variables|Default|SetCountdownTimer _returnvalue))
        (:then_1
          (if (< (Variables|Default|GetHiScore) _steps)
            (Variables|Default|SetHiScore _steps)
            (Default|UpdateHiScore (Variables|Default|GetHUDWidget))))))))

(fn IncreaseCoin
  (Math|Integer|IncrementInt (Variables|Default|GetCoins)
    (:%20%20
      (Default|UpdateCoinText (Variables|Default|GetHUDWidget)))))

(fn Restart
  (bind _returnvalue (Game|GetCurrentLevelName true))
  (Game|OpenLevel(byName) (Utilities|String|StringToName _returnvalue)))

(fn DisplayRestart
  (bind _returnvalue (Game|GetPlayerController 0))
  (bind _restartwidget (Variables|Default|GetRestartWidget))
  (if (UserInterface|Viewport|IsinViewport _restartwidget)
    _
    (else
      (UserInterface|Viewport|AddtoViewport _restartwidget 0)))
  (Input|SetInputModeUIOnly _returnvalue 0 "DoNotLock")
  (Variables|/Script/Engine.PlayerController|SetbShowMouseCursor _returnvalue true)
  (bind _returnvalue_2 (SaveGame|LoadGamefromSlot "save_data"))
  (bind _asbp_save_game (Utilities|Casting|CastToBP_SaveGame _returnvalue_2)
    (:then
      (Variables|Default|SetLocalSave _asbp_save_game))
    (:CastFailed
      (bind _returnvalue_3 (SaveGame|CreateSaveGameObject "/Game/Blueprints/BP_SaveGame.BP_SaveGame_C"))
      (bind _asbp_save_game_2 (Utilities|Casting|CastToBP_SaveGame _returnvalue_3))
      (Variables|Default|SetLocalSave _asbp_save_game_2)))
  (Variables|/Game/Blueprints/BP_SaveGame.BP_SaveGame_C|SetHiScore (Variables|Default|GetLocalSave) (Variables|Default|GetHiScore))
  (Variables|/Game/Blueprints/BP_SaveGame.BP_SaveGame_C|SetCoins (Variables|Default|GetLocalSave) (Variables|Default|GetCoins))
  (SaveGame|SaveGametoSlot (Variables|Default|GetLocalSave) "save_data"))

(fn PauseGame
  (bind _returnvalue (Game|GetPlayerController 0))
  (bind _pausewidget (Variables|Default|GetPauseWidget))
  (Development|PrintString "Pause")
  (Game|SetGamePaused true)
  (UserInterface|Viewport|AddtoViewport _pausewidget 0)
  (Input|SetInputModeUIOnly _returnvalue _pausewidget "DoNotLock")
  (Variables|/Script/Engine.PlayerController|SetbShowMouseCursor _returnvalue true))