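; Player chicken for a Crossy Road-style hopper: pressing a direction crouches, releasing hops and turns the mesh.
; Tick runs a LiveState machine for play and deaths (squashed, drowned, flushed away, eagle), which lead to the GameManager's restart display.
; Hops use manual gravity and swept interpolation, snapping Y to a grid on forward/back moves and reverting when blocked.
; New furthest X increments the step count; retreating too far triggers the eagle state, currently only a debug print.
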(event Custom|Rotate
  (bind _chickenmesh (Variables|Default|GetChickenMesh))
  (bind _desiredrotation (Variables|Default|GetDesiredRotation))
  (bind _returnvalue (Transformation|GetWorldRotation _chickenmesh))
  ;[1 1 1] Rotate
  (if (Utilities|Enum|NotEqual(Enum) _returnvalue _desiredrotation)
    (Transformation|SetWorldRotation (Variables|Default|GetChickenMesh) (Class|KismetMathLibrary|RInterptoConstant _returnvalue _desiredrotation (Utilities|Time|GetWorldDeltaSeconds) 5e+02) false false)))

(event Custom|Move
  (bind _returnvalue (Transformation|GetActorLocation))
  (bind _returnvalue_2 (Utilities|Time|GetWorldDeltaSeconds))
  (bind _returnvalue_3 (Transformation|GetActorLocation))
  (bind _endlocation (Variables|Default|GetEndLocation))
  (bind _endlocation_2 (Variables|Default|GetEndLocation))
  (bind _startlocation (Variables|Default|GetStartLocation))
  (bind _returnvalue_4 (Math|Interpolation|VInterptoConstant (Math|Vector|MakeVector (.x _returnvalue) (.y _returnvalue) 0.0) (Math|Vector|MakeVector (.x _endlocation_2) (.y _endlocation_2) 0.0) _returnvalue_2 1.2e+02))
  ;[1 1 1] Move
  (if (Variables|Default|GetIsMoving)
    (bind _returnvalue_5 (Transformation|SetActorLocation (Math|Vector|MakeVector (.x _returnvalue_4) (.y _returnvalue_4) (.z _returnvalue)) true false))
    (if _returnvalue_5
      (if (Math|Vector|Equal(Vector) (Math|Vector|MakeVector (.x _returnvalue_3) (.y _returnvalue_3) 0.0) (Math|Vector|MakeVector (.x _endlocation) (.y _endlocation) 0.0) 0.0001)
        (Variables|Default|SetIsMoving false)
        (if (Math|Vector|Equal(Vector) (Variables|Default|GetMoveDirection) (Class|KismetMathLibrary|VectorForward) 0.0001)
          (CallFunction|CheckHighestX)
          (elif (Math|Vector|Equal(Vector) (Variables|Default|GetMoveDirection) (* (Class|KismetMathLibrary|VectorForward) -1.0) 0.0001)
            (if (< (.x (Transformation|GetActorLocation)) (- (Variables|Default|GetHighestX) 8e+01))
              (CallFunction|SpawnEagle)))))
      (else
        (Transformation|SetActorLocation (Math|Vector|MakeVector (.x _startlocation) (.y _startlocation) (.z _returnvalue)) false false)
        (Variables|Default|SetIsMoving false)))))

(event Custom|UpdateGravity
  (bind _returnvalue (Utilities|Time|GetWorldDeltaSeconds))
  ;[1 1 1] Update Gravity
  (bind _output_get (Variables|Default|SetZSpeed (+ (Variables|Default|GetZSpeed) (* (Variables|Default|Getgravity) _returnvalue))))
  (bind _sweephitresult (Transformation|AddActorWorldOffset (Math|Vector|MakeVector 0.0 0.0 (* (Math|Float|Clamp(Float) _output_get -5e+02 5e+03) _returnvalue)) true))
  (if (.bBlockingHit (Collision|BreakHitResult _sweephitresult))
    (Variables|Default|SetIsJumping false)))

(event Custom|CheckHighestX
  (bind _returnvalue (Transformation|GetActorLocation))
  ;[1 1 1] Check location to increase step
  (if (> (.x _returnvalue) (Variables|Default|GetHighestX))
    (Default|IncreaseStep (Variables|Default|GetGameManager))
    (Variables|Default|SetHighestX (.x _returnvalue))))

(event Custom|FlushAway
  (params (Right :type Boolean))
  ;[1 1 1] Flush away
  (if Right
    (Variables|Default|SetLiveState 4)
    (else
      (Variables|Default|SetLiveState 5)))
  (Utilities|FlowControl|Delay 1.5)
  (Default|DisplayRestart (Variables|Default|GetGameManager)))

(event Custom|FlushRight
  (bind _chickenmesh (Variables|Default|GetChickenMesh))
  (bind _returnvalue (Transformation|GetWorldLocation _chickenmesh))
  ;[1 1 1] Flush
  (Transformation|SetWorldLocation _chickenmesh (Math|Vector|MakeVector (.x _returnvalue) (Math|Interpolation|FInterptoConstant (.y _returnvalue) 1e+03 (Utilities|Time|GetWorldDeltaSeconds) 4e+02) (.z _returnvalue)) false false))

(event Custom|FlushLeft
  (bind _chickenmesh (Variables|Default|GetChickenMesh))
  (bind _returnvalue (Transformation|GetWorldLocation _chickenmesh))
  ;[1 1 1] Flush
  (Transformation|SetWorldLocation _chickenmesh (Math|Vector|MakeVector (.x _returnvalue) (Math|Interpolation|FInterptoConstant (.y _returnvalue) -1e+03 (Utilities|Time|GetWorldDeltaSeconds) 4e+02) (.z _returnvalue)) false false))

(event Custom|AdjustY
  ;[1 1 1] Adjust End Location
  (Variables|Default|SetEndLocation (Math|Vector|MakeVector (.x (Variables|Default|GetEndLocation)) (* (Math|Float|Round (/ (.y (Variables|Default|GetEndLocation)) 4e+01)) 4e+01) (.z (Variables|Default|GetEndLocation)))))

(event Custom|SpawnEagle
  ;[1 1 1] Spawn Eagle
  (if (== (Variables|Default|GetLiveState) 0)
    (Variables|Default|SetLiveState 6)
    (Development|PrintString "Spawn Eagle")))

(event Custom|Crouch
  (bind _chickenmesh (Variables|Default|GetChickenMesh))
  (bind _chickenmesh_2 (Variables|Default|GetChickenMesh))
  (bind _chickenmesh_3 (Variables|Default|GetChickenMesh))
  (bind _relativescale3d (Variables|/Script/Engine.SceneComponent|GetRelativeScale3D _chickenmesh_2))
  (bind _relativescale3d_2 (Variables|/Script/Engine.SceneComponent|GetRelativeScale3D _chickenmesh_3))
  (if (Variables|Default|GetIsCrouching)
    (Transformation|SetRelativeScale3D _chickenmesh (Math|Vector|MakeVector (.x _relativescale3d_2) (.y _relativescale3d_2) (Math|Interpolation|FInterptoConstant (.z _relativescale3d_2) 0.7 (Utilities|Time|GetWorldDeltaSeconds) 5e+01)))
    (else
      (Transformation|SetRelativeScale3D _chickenmesh (Math|Vector|MakeVector (.x _relativescale3d) (.y _relativescale3d) (Math|Interpolation|FInterptoConstant (.z _relativescale3d) 1.0 (Utilities|Time|GetWorldDeltaSeconds) 8e+01))))))

(event EventBeginPlay
  ;[1 1 1] Begin
  (bind _returnvalue (Actor|GetActorOfClass "/Game/Blueprints/BP_GameManager.BP_GameManager_C"))
  (Variables|Default|SetGameManager _returnvalue)
  (Variables|Default|SetLiveState 0)
  (Variables|Default|SetIsJumping true)
  (Variables|Default|SetHighestX (.x (Transformation|GetActorLocation))))

(event EventTick
  (params (DeltaSeconds :type Float%20%28single-precision%29))
  ;[1 1 1] Main Update
  (switch int (Variables|Default|GetLiveState)
    (:0
      (CallFunction|UpdateGravity)
      (CallFunction|Rotate)
      (CallFunction|Crouch)
      (CallFunction|Move))
    (:1
      (Utilities|FlowControl|Delay 1.5 :!label _label)
      (Default|DisplayRestart (Variables|Default|GetGameManager)))
    (:2
      (CallFunction|UpdateGravity)
      (goto _label))
    (:4
      (CallFunction|FlushRight))
    (:5
      (CallFunction|FlushLeft))
    (:6
      (goto _label))))

(event Input|ActionEvents|InputActionMoveForward
  (params (Key :type Key%20Structure :default "None"))
  (bind _returnvalue (Transformation|GetActorLocation))
  ;[1 1 1] Input
  (:Pressed
    (if (not (Math|Boolean|ORBoolean (Variables|Default|GetIsMoving) (!= (Variables|Default|GetLiveState) 0) (Variables|Default|GetIsJumping)))
      (Variables|Default|SetIsCrouching true)))
  (:Released
    (if (not (Math|Boolean|ORBoolean (Variables|Default|GetIsMoving) (!= (Variables|Default|GetLiveState) 0) (Variables|Default|GetIsJumping)))
      (Variables|Default|SetMoveDirection (Class|KismetMathLibrary|VectorForward))
      (Variables|Default|SetDesiredRotation "0, 0, 0")
      (Pawn|Input|AddMovementInput (Variables|Default|GetMoveDirection) (Variables|Default|GetMoveDistance) false)
      (Variables|Default|SetIsMoving true)
      (Variables|Default|SetIsCrouching false)
      (Variables|Default|SetStartLocation _returnvalue)
      (bind _returnvalue_2 (Class|Pawn|ConsumeMovementInputVector))
      (Variables|Default|SetEndLocation (+ _returnvalue_2 _returnvalue))
      (if (or (Math|Vector|Equal(Vector) (Variables|Default|GetMoveDirection) (Class|KismetMathLibrary|VectorForward) 0.0001) (Math|Vector|Equal(Vector) (Variables|Default|GetMoveDirection) (* (Class|KismetMathLibrary|VectorForward) -1.0) 0.0001))
        (CallFunction|AdjustY))
      (Variables|Default|SetZSpeed 2.1e+02)
      (Variables|Default|SetIsJumping true))))

(event Input|ActionEvents|InputActionMoveLeft
  (params (Key :type Key%20Structure :default "None"))
  (bind _returnvalue (Transformation|GetActorLocation))
  ;[1 1 1] Input
  (:Pressed
    (if (not (Math|Boolean|ORBoolean (Variables|Default|GetIsMoving) (!= (Variables|Default|GetLiveState) 0) (Variables|Default|GetIsJumping)))
      (Variables|Default|SetIsCrouching true)))
  (:Released
    (if (not (Math|Boolean|ORBoolean (Variables|Default|GetIsMoving) (!= (Variables|Default|GetLiveState) 0) (Variables|Default|GetIsJumping)))
      (Variables|Default|SetMoveDirection (* (Class|KismetMathLibrary|VectorRight) -1.0))
      (Variables|Default|SetDesiredRotation "0,-90.000000, 0")
      (Pawn|Input|AddMovementInput (Variables|Default|GetMoveDirection) (Variables|Default|GetMoveDistance) false)
      (Variables|Default|SetIsMoving true)
      (Variables|Default|SetIsCrouching false)
      (Variables|Default|SetStartLocation _returnvalue)
      (bind _returnvalue_2 (Class|Pawn|ConsumeMovementInputVector))
      (Variables|Default|SetEndLocation (+ _returnvalue_2 _returnvalue))
      (if (or (Math|Vector|Equal(Vector) (Variables|Default|GetMoveDirection) (Class|KismetMathLibrary|VectorForward) 0.0001) (Math|Vector|Equal(Vector) (Variables|Default|GetMoveDirection) (* (Class|KismetMathLibrary|VectorForward) -1.0) 0.0001))
        (CallFunction|AdjustY))
      (Variables|Default|SetZSpeed 2.1e+02)
      (Variables|Default|SetIsJumping true))))

(event Input|ActionEvents|InputActionMoveRight
  (params (Key :type Key%20Structure :default "None"))
  (bind _returnvalue (Transformation|GetActorLocation))
  ;[1 1 1] Input
  (:Pressed
    (if (not (Math|Boolean|ORBoolean (Variables|Default|GetIsMoving) (!= (Variables|Default|GetLiveState) 0) (Variables|Default|GetIsJumping)))
      (Variables|Default|SetIsCrouching true)))
  (:Released
    (if (not (Math|Boolean|ORBoolean (Variables|Default|GetIsMoving) (!= (Variables|Default|GetLiveState) 0) (Variables|Default|GetIsJumping)))
      (Variables|Default|SetMoveDirection (Class|KismetMathLibrary|VectorRight))
      (Variables|Default|SetDesiredRotation "0,90.000000, 0")
      (Pawn|Input|AddMovementInput (Variables|Default|GetMoveDirection) (Variables|Default|GetMoveDistance) false)
      (Variables|Default|SetIsMoving true)
      (Variables|Default|SetIsCrouching false)
      (Variables|Default|SetStartLocation _returnvalue)
      (bind _returnvalue_2 (Class|Pawn|ConsumeMovementInputVector))
      (Variables|Default|SetEndLocation (+ _returnvalue_2 _returnvalue))
      (if (or (Math|Vector|Equal(Vector) (Variables|Default|GetMoveDirection) (Class|KismetMathLibrary|VectorForward) 0.0001) (Math|Vector|Equal(Vector) (Variables|Default|GetMoveDirection) (* (Class|KismetMathLibrary|VectorForward) -1.0) 0.0001))
        (CallFunction|AdjustY))
      (Variables|Default|SetZSpeed 2.1e+02)
      (Variables|Default|SetIsJumping true))))

(event Input|ActionEvents|InputActionMoveBack
  (params (Key :type Key%20Structure :default "None"))
  (bind _returnvalue (Transformation|GetActorLocation))
  ;[1 1 1] Input
  (:Pressed
    (if (not (Math|Boolean|ORBoolean (Variables|Default|GetIsMoving) (!= (Variables|Default|GetLiveState) 0) (Variables|Default|GetIsJumping)))
      (Variables|Default|SetIsCrouching true)))
  (:Released
    (if (not (Math|Boolean|ORBoolean (Variables|Default|GetIsMoving) (!= (Variables|Default|GetLiveState) 0) (Variables|Default|GetIsJumping)))
      (Variables|Default|SetMoveDirection (* (Class|KismetMathLibrary|VectorForward) -1.0))
      (Variables|Default|SetDesiredRotation "0,-180.000000,0.000000")
      (Pawn|Input|AddMovementInput (Variables|Default|GetMoveDirection) (Variables|Default|GetMoveDistance) false)
      (Variables|Default|SetIsMoving true)
      (Variables|Default|SetIsCrouching false)
      (Variables|Default|SetStartLocation _returnvalue)
      (bind _returnvalue_2 (Class|Pawn|ConsumeMovementInputVector))
      (Variables|Default|SetEndLocation (+ _returnvalue_2 _returnvalue))
      (if (or (Math|Vector|Equal(Vector) (Variables|Default|GetMoveDirection) (Class|KismetMathLibrary|VectorForward) 0.0001) (Math|Vector|Equal(Vector) (Variables|Default|GetMoveDirection) (* (Class|KismetMathLibrary|VectorForward) -1.0) 0.0001))
        (CallFunction|AdjustY))
      (Variables|Default|SetZSpeed 2.1e+02)
      (Variables|Default|SetIsJumping true))))

(event Input|ActionEvents|InputActionPause
  (params (Key :type Key%20Structure :default "None"))
  ;[1 1 1] Input
  (:Pressed
    (Default|PauseGame (Variables|Default|GetGameManager))))

(fn ConstructionScript)

(fn GetSquashedX
  (if (== (Variables|Default|GetLiveState) 0)
    (Transformation|SetRelativeScale3D (Variables|Default|GetChickenMesh) "0.100000,1.000000,1.000000")
    (Variables|Default|SetLiveState 1)))

(fn GetSquashedZ
  (if (== (Variables|Default|GetLiveState) 0)
    (Transformation|SetRelativeScale3D (Variables|Default|GetChickenMesh) "1.000000,1.000000,0.100000")
    (Variables|Default|SetLiveState 2)))

(fn Drown
  (if (== (Variables|Default|GetLiveState) 0)
    (Development|PrintString "Drown")
    (Variables|Default|SetLiveState 3)
    (Development|SetHiddeninGame (Variables|Default|GetChickenMesh) true false)
    (Effects|SpawnEmitteratLocation "/Game/Particles/P_Splash.P_Splash" (Transformation|GetActorLocation))
    (Default|DisplayRestart (Variables|Default|GetGameManager))))