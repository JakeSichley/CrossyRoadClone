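; BP_RoadLaneLeft is a road lane actor that endlessly spawns BP_Car traffic travelling in one direction.
; On BeginPlay it randomizes CarSpeed and waits a short random delay before the first spawn.
; SpawnCar creates a car at CarSpawnPoint, calls SetDirection with false, then calls itself again after a random delay.
; CarSpeed is not passed to the spawned cars in this graph.
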(event Custom|SpawnCar
  (bind _returnvalue (Game|SpawnActorfromClass "/Game/Blueprints/cars/BP_Car.BP_Car_C" (Transformation|GetWorldTransform (Variables|Default|GetCarSpawnPoint)) "Undefined" self 0))
  (Default|SetDirection _returnvalue false)
  (Utilities|FlowControl|Delay (Math|Random|RandomFloatinRange 3.5 7.0))
  (CallFunction|SpawnCar))

(event EventBeginPlay
  (|CallParentFunction)
  (Variables|Default|SetCarSpeed (Math|Random|RandomFloatinRange 5e+01 1.2e+02))
  (Utilities|FlowControl|Delay (Math|Random|RandomFloatinRange 0.0 3.0))
  (CallFunction|SpawnCar))

(event Collision|EventActorBeginOverlap
  (params (OtherActor :type Actor%20Object%20Reference)))

(event EventTick
  (params (DeltaSeconds :type Float%20%28single-precision%29))
  (|CallParentFunction DeltaSeconds) ; This node is disabled and will not be called.\nDrag off pins to build functionality.
)

(fn ConstructionScript
  (|CallParentFunction))