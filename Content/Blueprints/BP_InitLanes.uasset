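; BP_InitLanes is a lane actor that fills a row with random static meshes and removes itself once the player has moved past it.
; BeginPlay caches BP_Player, then adds fifteen evenly spaced mesh components along Y, each through one of three randomly picked branches with identical offsets.
; Tick compares the player's Box to the actor root along X and destroys the actor when the player is far enough ahead.
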(event EventBeginPlay
  (bind _returnvalue (Actor|GetActorOfClass "/Game/Blueprints/BP_Player.BP_Player_C"))
  (Variables|Default|SetPlayer _returnvalue)
  (for _index (range -7 7)
    (switch int (Math|Random|RandomIntegerinRange 0 2)
      (:Default
        (AddComponent|AddStaticMeshComponent false (Math|Transform|MakeTransform (Math|Vector|MakeVector 2e+01 (* _index 4e+01) 4.0) "0, 0, 0" "1,1,1") :!label _label))
      (:0
        (AddComponent|AddStaticMeshComponent false (Math|Transform|MakeTransform (Math|Vector|MakeVector 2e+01 (* _index 4e+01) 4.0) "0, 0, 0" "1,1,1")))
      (:1
        (AddComponent|AddStaticMeshComponent false (Math|Transform|MakeTransform (Math|Vector|MakeVector 2e+01 (* _index 4e+01) 4.0) "0, 0, 0" "1,1,1")))
      (:2
        (goto _label)))))

(event EventTick
  (params (DeltaSeconds :type Float%20%28single-precision%29))
  (if (> (- (.x (Transformation|GetWorldLocation (Variables|/Game/Blueprints/BP_Player.BP_Player_C|GetBox (Variables|Default|GetPlayer)))) (.x (Transformation|GetWorldLocation (Variables|Default|GetDefaultSceneRoot)))) 2.6e+02)
    (Actor|DestroyActor)))

(fn ConstructionScript)